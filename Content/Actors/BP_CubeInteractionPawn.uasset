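; BP_CubeInteractionPawn is an interactable pawn that a character can take control of.
; When interaction completes, it has the interacting character's controller possess it.
; The Unpossess input releases this pawn, calls Possess on the interactor through that character's GetController, and re-enables query and physics collision on its capsule and mesh.
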(event `InteractableInterface.OnInteractionCompleted`
  (`self.Possess` (`self.GetController` (`self.BeingInteractedBy`))))

(event `InputAction|Unpossess`
  (params (Key :type "Key Structure"))
  (bind _beinginteractedby (`self.BeingInteractedBy`))
  (:`Pressed`
    (`Controller.UnPossess` (`self.GetController`))
    (`Controller.Possess` (`self.GetController` _beinginteractedby) _beinginteractedby)
    (`PrimitiveComponent.SetCollisionEnabled` (`Character.CapsuleComponent` _beinginteractedby) "QueryAndPhysics")
    (`PrimitiveComponent.SetCollisionEnabled` (`Character.Mesh` _beinginteractedby) "QueryAndPhysics")))

(fn `Possess`
  (params (Controller :type "Controller Object Reference"))
  (`Controller.Possess` Controller self))

(fn `UserConstructionScript`)