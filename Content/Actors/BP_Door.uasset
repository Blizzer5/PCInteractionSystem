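; BP_Door is an interactable door that toggles between open and closed when an interaction completes.
; The OpenCloseDoor timeline plays forward or in reverse based on IsOpen, setting the whole actor's absolute yaw from its CurrentAngle track.
; Interaction is disabled during the swing; on finish, the door flips IsOpen, switches the action name between Open and Close, and re-enables interaction.
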(event `InteractableInterface.OnInteractionCompleted`
  (`InteractableInterface.DisableInteraction`)
  (if (`self.bIsOpen`)
    (bind (_direction _currentangle) (`Timeline|OpenCloseDoor` :!via `Reverse` :!label _label)
      (:`Update`
        (`self.K2_SetActorRotation` (`KismetMathLibrary.MakeRotator` (.roll (`self.K2_GetActorRotation`)) (.pitch (`self.K2_GetActorRotation`)) _currentangle)))
      (:`Finished`
        (set `self.bIsOpen` (not (`self.bIsOpen`)))
        (`InteractableInterface.SetInteractionActionName` (`|FormatText` (select `bool` (`self.bIsOpen`) :`false` "Open" :`true` "Close" :!type "Text")))
        (`InteractableInterface.EnableInteraction`)))
    (else
      (goto _label))))

(fn `UserConstructionScript`)